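; Player tank pawn Blueprint that handles camera aiming and firing input.
; BeginPlay passes the Turret and Barrel components to the parent's reference setters.
; Aim axes rotate a HorizontalAzimuth component for yaw and the SpringArm for pitch, scaled by frame delta time, to orbit the third-person camera.
; The fire action calls Fire, whose logic is not defined in this graph.
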(event `self.ReceiveBeginPlay`
  (`self.SetTurretReference` (`self.Turret`))
  (`self.SetBarrelReference` (`self.Barrel`)))

(event `InputAxis|AimAzimuthElevation`
  (params (AxisValue :type "Float (single-precision)"))
  (`SceneComponent.K2_AddLocalRotation` (`self.SpringArm`) (`KismetMathLibrary.MakeRotator` 0.0 (* AxisValue (`GameplayStatics.GetWorldDeltaSeconds`) 100.0)) false false))

(event `InputAxis|AimAzimuthHorizontal`
  (params (AxisValue :type "Float (single-precision)"))
  (`SceneComponent.K2_AddLocalRotation` (`self.HorizontalAzimuth`) (`KismetMathLibrary.MakeRotator` 0.0 0.0 (* AxisValue (`GameplayStatics.GetWorldDeltaSeconds`) 100.0)) false false))

(event `InputAction|PlayerTankFiring`
  (params (Key :type "Key Structure" :default "AnyKey"))
  (:`Pressed`
    (`self.Fire`)))

(fn `UserConstructionScript`)